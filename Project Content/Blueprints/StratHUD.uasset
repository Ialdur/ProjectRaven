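; StratHUD is a HUD Blueprint that draws a pause menu with Resume and Quit buttons around the screen center.
; While MenuOpen is true, DrawHUD calls the DrawButton helper to render each textured, labeled button with a named hit box.
; HitBoxClick matches those names to close the menu and unpause, or quit the game.
; Tick re-applies pause every frame while the menu is open.
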(event EventDrawHUD
  (params (SizeX :type Integer) (SizeY :type Integer))
  (bind _returnvalue (Math|Conversions|ToFloat(Integer) SizeY))
  (bind _returnvalue_2 (Math|Conversions|ToFloat(Integer) SizeX))
  (bind _returnvalue_3 (Math|Vector2D|MakeVector2D _returnvalue_2 _returnvalue))
  (bind _returnvalue_4 (/ _returnvalue_3 2.0))
  (bind (_x _y) (Math|Vector2D|BreakVector2D _returnvalue_4))
  ;[1 1 1] Draw Menu
  (if (Variables|Default|GetMenuOpen)
    (CallFunction|DrawButton _x (+ _y -1e+02) 1e+02 1e+02 1e+01 25.0 "Resume")
    (CallFunction|DrawButton _x (+ _y 1e+02) 1e+02 1e+02 2e+01 25.0 "Quit")))

(event EventGetMousePosition
  (params (Mouse%20Position :type Vector%202D%20Structure))
  ;[1 1 1] Setting/getting state variables
)

(event EventToggleMenu
  (params (Menu%20open :type Boolean))
  ;[1 1 1] Setting/getting state variables
  (if (not (Variables|Default|GetMenuOpen))
    (Variables|Default|SetMenuOpen Menu%20open)))

(event EventHitBoxClick
  (params (BoxName :type Name :default "None"))
  ;[1 1 1] Draw Menu
  (if (Utilities|Name|Equal(Name) BoxName "Resume")
    (Variables|Default|SetMenuOpen false)
    (Game|SetGamePaused false)
    (elif (Utilities|Name|Equal(Name) BoxName "Quit")
      (Game|QuitGame (Game|GetPlayerController 0) "Quit"))))

(event EventBeginPlay
  ;[1 1 1] Setting/getting state variables
  (Variables|Default|SetMenuOpen false))

(event EventTick
  (params (DeltaSeconds :type Float%20%28single-precision%29))
  ;[1 1 1] Enable Pausing if forced
  (if (Variables|Default|GetMenuOpen)
    (Game|SetGamePaused true)))

(fn ConstructionScript)

(fn DrawButton
  (params (PosX :type Float%20%28single-precision%29 :default 0.0) (PosY :type Float%20%28single-precision%29 :default 0.0) (Width :type Float%20%28single-precision%29 :default 0.0) (Height :type Float%20%28single-precision%29 :default 0.0) (FontOffsetW :type Float%20%28single-precision%29 :default 0.0) (FontOffsetH :type Float%20%28single-precision%29 :default 0.0) (Buttonname :type Name :default "None"))
  (Canvas|DrawTexture "/Game/StarterContent/Textures/T_Wood_Walnut_D.T_Wood_Walnut_D" PosX PosY Width Height 0.0 0.0 1.0 1.0 "(R=1.000000,G=1.000000,B=1.000000,A=1.000000)" "BLEND_Masked")
  (HUD|DrawText (Utilities|String|ToString(Name) Buttonname) "(R=1.000000,G=1.000000,B=1.000000,A=1.000000)" (+ PosX FontOffsetW) (+ PosY FontOffsetH) "/Game/Fonts/StratFont.StratFont" 0.3 false)
  (Class|HUD|AddHitBox (Math|Vector2D|MakeVector2D PosX PosY) (Math|Vector2D|MakeVector2D Width Height) Buttonname false 3))