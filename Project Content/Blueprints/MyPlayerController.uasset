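; Player controller for a top-down style camera, with mouse edge scrolling, wheel zoom and a HUD menu toggle.
; Each tick it turns screen-edge hits into normalized, frame-rate-scaled movement, then traces down to the ground to hold the target above the terrain.
; Wheel input adjusts spring arm length, smoothed by a lerp and clamped to distance limits.
; The resulting transform and arm length are sent to the pawn by message.
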(event EventTick
  (params (DeltaSeconds :type Float%20%28single-precision%29))
  ;[1 1 1] Main Function / Event Tick
  (bind _pawntransformrefresh (CallFunction|CameraMovement))
  (CallFunction|CameraZoom)
  (bind _output_get (Variables|Default|SetPawnTransformRefresh _pawntransformrefresh))
  (Class|PlayerControlInterface|SendPlayerControllerData(Message) (Game|Player|GetPlayerPawn 0) _output_get (Variables|Default|GetSpringArmLengthRefresh)))

(event EventBeginPlay
  ;[1 1 1] Declerations on Startup
  (Input|EnableInput self)
  (Variables|Default|SetPawnTransformRefresh (Transformation|GetActorTransform (Game|Player|GetPlayerPawn 0))) ; Set the local PawnTransformRefresh \nto the Transform of the Pawn. This will \nprevent refreshing the Pawn to the Position \n(0 / 0 / 0) at start.
)

(event Input|ActionEvents|InputActionMenu
  ;[1 1 1] Menu Trigger
  (:Pressed
    (Class|StratHUDInterface|ToggleMenu(Message) (HUD|GetHUD) true)))

(event Input|ActionEvents|InputActionMouseWheelDown
  ;[1 1 1] Camera Zoom
  (:Pressed
    (Variables|Default|SetNewSpringArmLenght (+ (Variables|Default|GetNewSpringArmLenght) (Variables|Default|GetZoomSpeed)))))

(event Input|ActionEvents|InputActionMouseWheelUp
  ;[1 1 1] Camera Zoom
  (:Pressed
    (Variables|Default|SetNewSpringArmLenght (- (Variables|Default|GetNewSpringArmLenght) (Variables|Default|GetZoomSpeed)))))

(fn ConstructionScript
  (Variables|Default|SetScreenResolution (Viewport|GetViewportSize)) ; Set the ScreenResolution Variable \nto the Viewport Size.\n-----------------------------------\n!!! Still a bit Buggy, suggest a different \nway to get the Screen Resolution !!!
)

(fn SetHorizontalMovement
  (params (AxisValue :type Float%20%28single-precision%29 :default 0.0))
  (bind _movement (Variables|Default|GetMovement))
  (bind (_x _y _z) (Math|Vector|BreakVector _movement))
  (return (Math|Vector|MakeVector _x AxisValue _z)))

(fn SetVerticalMovement
  (params (AxisValue :type Float%20%28single-precision%29 :default 0.0))
  (bind _movement (Variables|Default|GetMovement))
  (bind (_x _y _z) (Math|Vector|BreakVector _movement))
  (return (Math|Vector|MakeVector AxisValue _y _z)))

(fn IsMouseinScrollArea
  (params (MouseX :type Float%20%28single-precision%29 :default 0.0) (MouseY :type Float%20%28single-precision%29 :default 0.0))
  (bind _screenresolution (Variables|Default|GetScreenResolution))
  (bind _scrollareawidth (Variables|Default|GetScrollAreaWidth))
  (bind (_x _y) (Math|Vector2D|BreakVector2D _screenresolution))
  (bind (_x_2 _y_2) (Math|Vector2D|BreakVector2D _scrollareawidth))
  (return (> MouseX (- _x _x_2)) (< MouseX _x_2) (> MouseY (- _y _y_2)) (< MouseY _y_2)))

(fn MovementtoTransformRefresh
  (bind _returnvalue (Utilities|Time|GetWorldDeltaSeconds))
  (bind _movement (Variables|Default|GetMovement))
  (bind _pawntransformrefresh (Variables|Default|GetPawnTransformRefresh))
  (bind _scrollspeed (Variables|Default|GetScrollSpeed))
  (bind (_location _rotation _scale) (Math|Transform|BreakTransform _pawntransformrefresh))
  (bind _returnvalue_2 (Math|Vector|Normalize _movement))
  (bind _returnvalue_3 (* _scrollspeed _returnvalue))
  (bind _returnvalue_4 (* _returnvalue_2 _returnvalue_3))
  (bind _returnvalue_5 (Math|Transform|TransformDirection _pawntransformrefresh _returnvalue_4))
  (bind _returnvalue_6 (+ _returnvalue_5 _location))
  (bind (_x _y) (Math|Vector|BreakVector _returnvalue_6))
  (bind (_outhit _returnvalue_7) (Collision|LineTraceByChannel _returnvalue_6 (Math|Vector|MakeVector _x _y -1e+03) "TraceTypeQuery1" false 0 "None")) ; Cast a Raycast to the surface of th desired position
  (if _returnvalue_7 ; If it hits something, there is a surface so \nwe can move
    (return (Math|Transform|MakeTransform (Math|Vector|MakeVector (.X (Math|Vector|BreakVector (.Location (Collision|BreakHitResult _outhit)))) (.Y (Math|Vector|BreakVector (.Location (Collision|BreakHitResult _outhit)))) (+ (.Z (Math|Vector|BreakVector (.Location (Collision|BreakHitResult _outhit)))) 1e+02)) _rotation _scale))))

(fn CameraMovement
  (bind (_locationx _locationy) (Game|Player|GetMousePosition))
  (bind (_rightx _leftx _bottomy _topy) (CallFunction|IsMouseinScrollArea _locationx _locationy)) ; Check if the mouse at the edge of \nthe Screen. In relation at which edge \nthe mouse hits the screen edge, \ncall the different functions
  (if _rightx
    (bind _horizontalmovement (CallFunction|SetHorizontalMovement 1.0))
    (Variables|Default|SetMovement _horizontalmovement)
    (elif _leftx
      (bind _horizontalmovement_2 (CallFunction|SetHorizontalMovement -1.0))
      (Variables|Default|SetMovement _horizontalmovement_2)))
  (if _bottomy
    (bind _verticalmovement (CallFunction|SetVerticalMovement -1.0))
    (Variables|Default|SetMovement _verticalmovement)
    (elif _topy
      (bind _verticalmovement_2 (CallFunction|SetVerticalMovement 1.0))
      (Variables|Default|SetMovement _verticalmovement_2)))
  (bind _transformrefresh (CallFunction|MovementtoTransformRefresh))
  (Variables|Default|SetMovement "0, 0, 0")
  (return _transformrefresh))

(fn CameraZoom
  (bind _output_get (Variables|Default|SetSpringArmLengthRefresh (Math|Float|Clamp(Float) (Math|Float|Lerp (Variables|Default|GetSpringArmLengthRefresh) (Variables|Default|GetNewSpringArmLenght) 0.5) (Variables|Default|GetMinCameraDistance) (Variables|Default|GetMaxCameraDistance))))
  (Variables|Default|SetNewSpringArmLenght _output_get))